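; BP_FrogSpawner is a quest-driven spawner that places BP_Frog actors in the world when its QuestReaction reports that requirements are met.
; The construction script gathers five box areas into the SpawnAreas array.
; On that event, a loop driven by FrogsToSpawn spawns frogs with random yaw at random points within randomly picked areas, using half the scaled box extent to keep them toward the centre.
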(event `self.QuestReaction.OnRequirementsMet`
  (params (Sender :type "QuestReactionComponent Object Reference"))
  (bind _outitem (`KismetArrayLibrary.Array_Random` (`self.SpawnAreas`)))
  (for _ (range (+ (`self.FrogsToSpawn`) 1))
    (`|SpawnActorFromClass` "/Game/Actors/Frog/BP_Frog.BP_Frog_C" (`KismetMathLibrary.MakeTransform` (`KismetMathLibrary.RandomPointInBoundingBox` (`SceneComponent.K2_GetComponentLocation` _outitem) (* (`BoxComponent.GetScaledBoxExtent` _outitem) 0.5)) (`KismetMathLibrary.MakeRotator` 0.0 0.0 (`KismetMathLibrary.RandomFloatInRange` -180.0 180.0))) "Undefined" "OverrideRootScale" null null)))

(fn `UserConstructionScript`
  (`KismetArrayLibrary.Array_Add` (`self.SpawnAreas`) (`self.SpawnArea01`))
  (`KismetArrayLibrary.Array_Add` (`self.SpawnAreas`) (`self.SpawnArea02`))
  (`KismetArrayLibrary.Array_Add` (`self.SpawnAreas`) (`self.SpawnArea03`))
  (`KismetArrayLibrary.Array_Add` (`self.SpawnAreas`) (`self.SpawnArea04`))
  (`KismetArrayLibrary.Array_Add` (`self.SpawnAreas`) (`self.SpawnArea05`)))
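; BP_BeachFrogComponent makes frogs scannable inside an overlap area while the Q_FrogBeach quest is active.
; On begin overlap it checks the quest subsystem, casts the other actor to BP_Frog and enables that frog's Scannable.
; On end overlap it disables Scannable again, also only while the quest is active.
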(event `self.OnActorBeginOverlap`
  (params (OverlappedActor :type "Actor Object Reference") (OtherActor :type "Actor Object Reference"))
  (if (`QuestSubsystem.IsQuestActive` (subsystem `QuestSubsystem`) "/Game/Quests/Q_FrogBeach.Q_FrogBeach")
    (bind _asbp_frog (cast `/Game/Actors/Frog/BP_Frog` OtherActor))
    (`ScannableComponent.Enable` (`/Game/Actors/Frog/BP_Frog.Scannable` _asbp_frog))))

(event `self.OnActorEndOverlap`
  (params (OverlappedActor :type "Actor Object Reference") (OtherActor :type "Actor Object Reference"))
  (if (`QuestSubsystem.IsQuestActive` (subsystem `QuestSubsystem`) "/Game/Quests/Q_FrogBeach.Q_FrogBeach")
    (bind _asbp_frog (cast `/Game/Actors/Frog/BP_Frog` OtherActor))
    (`ScannableComponent.Disable` (`/Game/Actors/Frog/BP_Frog.Scannable` _asbp_frog))))
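; Handheld camera item that the main character picks up through interaction, which adds it to the inventory and sets its owning pawn.
; Overrides the parent's aim, offhand and holster events to pose and attach it to the hand root or detach it.
; Aiming narrows or changes the player's target FOV and enables vignette and focal distance post-processing, which the other states reset.
; Taking a picture calls the parent logic and plays a flash sound.
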(event `self.InteractableComponent.OnInteractionComplete`
  (params (Sender :type "HermesInteractableComponent Object Reference") (Instigator :type "Actor Object Reference"))
  (`PrimitiveComponent.SetCollisionEnabled` (`self.InteractableComponent`) "NoCollision")
  (bind _asmain_character (cast `MainCharacter` Instigator))
  (`InventoryComponent.AddItem` (`MainCharacter.GetInventory` _asmain_character) self)
  (`self.SetOwningPawn` _asmain_character))

(event `self.OnPictureTaken`
  (params (bSuccess :type Boolean) (ScannableComponent :type "ScannableComponent Object Reference"))
  (`parent.OnPictureTaken` bSuccess ScannableComponent)
  (`GameplayStatics.PlaySoundAtLocation` "/Game/Audio/Camera/C_CameraFlash.C_CameraFlash" (`self.K2_GetActorLocation`) (struct) 1.0 1.0 0.0 null null null null))

(event `self.OnAim`
  (params (InInstigator :type "Controller Object Reference"))
  (`parent.OnAim` InInstigator)
  (`self.K2_SetActorRelativeTransform` (`KismetMathLibrary.MakeTransform` (16.0 0.0 -7.0) (struct :`Yaw` 90.0) (0.1 0.1 0.1)))
  (bind _asmain_character (cast `MainCharacter` (`Controller.K2_GetPawn` InInstigator)))
  (`MainCharacter.SetTargetFov` _asmain_character (`self.CameraFov`) false)
  (bind _returnvalue (`MainCharacter.GetHandRoot` _asmain_character))
  (`SceneComponent.K2_SetRelativeLocation` _returnvalue (0.0 -3.5 0.0) false false)
  (`self.K2_AttachToComponent` _returnvalue "None" "KeepRelative" "KeepRelative" "KeepRelative")
  (`self.EnablePlayerCameraPostProcessing` _asmain_character))

(event `self.OnOffhand`
  (params (InInstigator :type "Controller Object Reference"))
  (`parent.OnOffhand` InInstigator)
  (`self.K2_SetActorRelativeTransform` (`KismetMathLibrary.MakeTransform` (24.0 0.0 -12.0) (struct :`Yaw` 90.0 :`Roll` 15.0) (0.1 0.1 0.1)))
  (bind _asmain_character (cast `MainCharacter` (`Controller.K2_GetPawn` InInstigator)))
  (`self.ResetPlayer` _asmain_character)
  (`self.K2_AttachToComponent` (`MainCharacter.GetHandRoot` _asmain_character) "None" "KeepRelative" "KeepRelative" "KeepRelative"))

(event `self.OnHolstered`
  (params (InInstigator :type "Controller Object Reference"))
  (`parent.OnHolstered` InInstigator)
  (`self.K2_DetachFromActor` "KeepRelative")
  (bind _asmain_character (cast `MainCharacter` (`Controller.K2_GetPawn` InInstigator)))
  (`self.ResetPlayer` _asmain_character))

(event `EnablePlayerCameraPostProcessing`
  (params (Char :type "MainCharacter Object Reference"))
  (setmembers `PostProcessSettings` :`StructRef` (`CameraComponent.PostProcessSettings` (`FrogwaterCharacter.FirstPersonCameraComponent` Char)) :`VignetteIntensity` 1.0 :`DepthOfFieldFocalDistance` 10.65))

(event `DisablePlayerCameraPostProcessing`
  (params (Char :type "MainCharacter Object Reference"))
  (setmembers `PostProcessSettings` :`StructRef` (`CameraComponent.PostProcessSettings` (`FrogwaterCharacter.FirstPersonCameraComponent` Char)) :`VignetteIntensity` 0.0 :`DepthOfFieldFocalDistance` 0.0))

(event `ResetPlayer`
  (params (Char :type "MainCharacter Object Reference"))
  (`MainCharacter.ResetTargetFov` Char false)
  (`MainCharacter.ResetTargetFov` Char false)
  (`SceneComponent.K2_SetRelativeLocation` (`MainCharacter.GetHandRoot` Char) (0.0 0.0 0.0) false false)
  (`self.DisablePlayerCameraPostProcessing` Char))

(fn `UserConstructionScript`)
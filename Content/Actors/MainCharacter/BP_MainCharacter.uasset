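; First-person main character Blueprint that starts quests, prints interaction feedback and handles physics carrying of frogs.
; BeginPlay adds the church secret quest and, after a delay, the grandma's house quest.
; Frog hand items are grabbed by a stiff physics handle following the hand root each tick, and released on switching.
; Footsteps alternate by horizontal velocity accumulation instead of animation notifies; Tab temporarily shows a test scrapbook widget.
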(event `Key|Tab`
  (params (Key :type "Key Structure"))
  (bind _test_scrapbookwidget (`self.TEST_ScrapbookWidget`))
  ;[1 0 0.1187] TEMP _ REMOVE
  (:`Pressed`
    (bind _asplayer_controller (cast `PlayerController` (`self.GetController`)))
    (bind _returnvalue (`|CreateWidget` "/Game/CharacterTest/WB_LoadPictureTest.WB_LoadPictureTest_C" _asplayer_controller))
    (set `self.TEST_ScrapbookWidget` _returnvalue)
    (`UserWidget.AddToPlayerScreen` _returnvalue 0))
  (:`Released`
    (`/Engine/EditorBlueprintResources/StandardMacros.IsValid` _test_scrapbookwidget
      (:`Is Valid`
        (`Widget.RemoveFromParent` _test_scrapbookwidget)))))

(event `self.ReceiveBeginPlay`
  (bind _pickupphysicshandle (`self.PickupPhysicsHandle`))
  (`self.Add Intro Quest`)
  (`PhysicsHandleComponent.SetInterpolationSpeed` _pickupphysicshandle 2000.0)
  (`PhysicsHandleComponent.SetLinearDamping` _pickupphysicshandle 0.0)
  (`PhysicsHandleComponent.SetLinearStiffness` _pickupphysicshandle 6000.0)
  (`QuestSubsystem.AddQuest` (subsystem `QuestSubsystem`) "/Game/Quests/Q_Secret_Church.Q_Secret_Church"))

(event `self.ReceiveTick`
  (params (DeltaSeconds :type "Float (single-precision)"))
  (bind _returnvalue (`self.GetHandRoot`))
  (`self.UpdateFootsteps`)
  (`PhysicsHandleComponent.SetTargetLocation` (`self.PickupPhysicsHandle`) (+ (`SceneComponent.K2_GetComponentLocation` _returnvalue) (* (`SceneComponent.GetForwardVector` _returnvalue) 50.0) (* (`SceneComponent.GetUpVector` _returnvalue) -10.0))))

(event `Add Intro Quest`
  (`KismetSystemLibrary.Delay` 4.0)
  (`QuestSubsystem.AddQuest` (subsystem `QuestSubsystem`) "/Game/Quests/Q_GrandmasHouse.Q_GrandmasHouse"))

(event `self.InteractorComponent.OnFocus`
  (params (Sender :type "HermesInteractorComponent Object Reference") (InteractableComponent :type "HermesInteractableComponent Object Reference"))
  (`KismetSystemLibrary.PrintString` (`KismetTextLibrary.Conv_TextToString` (`HermesInteractableComponent.GetFocusText` InteractableComponent))))

(event `self.InteractorComponent.OnInteractionStarted`
  (params (Sender :type "HermesInteractorComponent Object Reference") (InteractableComponent :type "HermesInteractableComponent Object Reference"))
  (`KismetSystemLibrary.PrintString` (`KismetTextLibrary.Conv_TextToString` (`HermesInteractableComponent.GetInteractingText` InteractableComponent))))

(event `self.InteractorComponent.OnInteractionComplete`
  (params (Sender :type "HermesInteractorComponent Object Reference") (InteractableComponent :type "HermesInteractableComponent Object Reference"))
  (`KismetSystemLibrary.PrintString` "Picked up"))

(event `UpdateFootsteps`
  ;[1 1 1] Would be more accurate to use animation steps but don't have any coz first person
  (bind _output_get (set `self.RemainingFootDistance` (- (`self.RemainingFootDistance`) (`KismetMathLibrary.VSizeXY` (`self.GetVelocity`)))))
  (if (<= _output_get 0.0)
    (`self.OnFootDistanceReached`)))

(event `OnFootDistanceReached`
  ;[1 1 1] Would be more accurate to use animation steps but don't have any coz first person
  (set `self.RemainingFootDistance` (`self.FootTravelDistance`))
  (set `self.bIsLeftFoot` (not (`self.bIsLeftFoot`)))
  (`BFFootstepsComponent.CalculateAndPlay` (`self.FootstepsComponent`) (`KismetMathLibrary.VSizeXY` (`self.GetVelocity`)) (`KismetMathLibrary.SelectInt` 0 1 (`self.bIsLeftFoot`))))

(event `self.InventoryComponent.OnHandItemChanged`
  (params (Sender :type "CharacterInventoryComponent Object Reference") (NewItem :type "Actor Object Reference") (NewHandItemIndex :type Integer) (PreviousItem :type "Actor Object Reference") (PreviousHandItemIndex :type Integer))
  (bind _asbp_frog (cast `/Game/Actors/Frog/BP_Frog` NewItem)
    (:`then`
      (bind _staticmesh (`/Game/Actors/Frog/BP_Frog.StaticMesh` _asbp_frog))
      (bind _output_get (set `self.PhysicsComponent` _staticmesh))
      (`PhysicsHandleComponent.GrabComponentAtLocation` (`self.PickupPhysicsHandle`) _output_get "None" (`SceneComponent.K2_GetComponentLocation` _staticmesh)))
    (:`CastFailed`
      (cast `/Game/Actors/Frog/BP_Frog` PreviousItem)
      (`PhysicsHandleComponent.ReleaseComponent` (`self.PickupPhysicsHandle`))
      (set `self.PhysicsComponent` null))))

(fn `UserConstructionScript`
  (bind _footstepscomponent (`self.FootstepsComponent`))
  (bind _mesh (`self.Mesh`))
  (`BFFootstepsComponent.AddFootUsingSocket` _footstepscomponent _mesh "foot_l" 1.0)
  (`BFFootstepsComponent.AddFootUsingSocket` _footstepscomponent _mesh "foot_r" 1.0))
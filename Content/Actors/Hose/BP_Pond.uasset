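; Pond actor that rises as it is filled and completes the Fill The Pond quest once full.
; Each Fill call nudges the actor up by a fixed step until it reaches the target height above its construction-time Z; a further call then completes the quest through the Quest subsystem.
; Filled is set only if that completion succeeds, so later calls can retry and avoid a soft lock.
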(event `Fill`
  (bind (_returnvalue_x _returnvalue_y _returnvalue_z) (`KismetMathLibrary.BreakVector` (`self.K2_GetActorLocation`)))
  (if (not (`self.Filled`))
    (if (>= _returnvalue_z (+ (`self.InitialHeight`) (`self.FilledHeight`)))
      ;[1 1 1] Pond filled
      (`self.Complete Quest`)
      (else
        (`self.K2_AddActorLocalOffset` (`KismetMathLibrary.MakeVector` 0.0 0.0 (`self.HeightPerHit`)))))))

(event `Complete Quest`
  (bind _returnvalue (`QuestSubsystem.CompleteQuest` (subsystem `QuestSubsystem`) "/Game/Quests/Q_FillThePond.Q_FillThePond"))
  (set `self.Filled` _returnvalue) ; Only set filled if the Quest was found and completed (no soft locking)
)

(fn `UserConstructionScript`
  (bind (_returnvalue_x _returnvalue_y _returnvalue_z) (`KismetMathLibrary.BreakVector` (`self.K2_GetActorLocation`)))
  (set `self.InitialHeight` _returnvalue_z))
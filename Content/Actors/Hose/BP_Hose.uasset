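; BP_Hose is a carryable hose that the player picks up as an inventory item and sprays with Niagara to fill a pond.
; While held, Tick pins the nozzle to the player's right hand and view rotation, auto-dropping it as a physics object past maximum length.
; Niagara exports particle data back to the Blueprint, which fills PondRef for sampled particles inside its box.
; The construction script configures the cable and callback.
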(event `self.ReceiveBeginPlay`
  (add `self.MaxLengthReached` (delegate `MaxLengthReached_Event`)))

(event `MaxLengthReached_Event` :!signature `self.MaxLengthReached`
  (params (Sender :type "/Game/Actors/Hose/BP_Hose Object Reference"))
  (`KismetSystemLibrary.PrintString` "Max Length Reached"))

(event `self.ReceiveTick`
  (params (DeltaSeconds :type "Float (single-precision)"))
  (bind _hosetip (`self.HoseTip`))
  (bind _character (`self.Character`))
  ;[1 1 1] Check if over max length
  (if (>= (`KismetMathLibrary.Vector_Distance` (`SceneComponent.K2_GetComponentLocation` (`self.HoseTip`)) (`SceneComponent.K2_GetComponentLocation` (`self.HoseBarrel`))) (`self.Length`))
    (`self.MaxLengthReached` self)
    (`/Engine/EditorBlueprintResources/StandardMacros.IsValid` (`self.Character`)
      (:`Is Valid`
        (`self.DropHose`)
        ;[1 1 1] Move the hose back a bit so it can be re-picked up
        (`SceneComponent.K2_SetWorldLocation` (`self.HoseTip`) (`KismetMathLibrary.VLerp` (`SceneComponent.K2_GetComponentLocation` (`self.HoseTip`)) (`SceneComponent.K2_GetComponentLocation` (`self.HoseBarrel`)) 0.2) true false)))
    (else
      ;[1 1 1] Set location and transform of hose nozzle to player hand
      (`/Engine/EditorBlueprintResources/StandardMacros.IsValid` _character
        (:`Is Valid`
          (`SceneComponent.K2_SetWorldLocation` _hosetip (`SceneComponent.K2_GetComponentLocation` (`MainCharacter.GetRightHand` _character)) false false)
          (`SceneComponent.K2_SetWorldRotation` _hosetip (`FrogwaterStatics.AddRotator` (`.OutRotation` (`self.GetActorEyesViewPoint` _character)) (`KismetMathLibrary.MakeRotator` 0.0 110.0)) false false))))))

(event `self.OnOffhand`
  (params (InInstigator :type "Controller Object Reference")))

(event `self.HermesInteractable.OnInteractionComplete`
  (params (Sender :type "HermesInteractableComponent Object Reference") (Instigator :type "Actor Object Reference"))
  (bind _hosetip (`self.HoseTip`))
  (`PrimitiveComponent.SetCollisionEnabled` (`self.HermesInteractable`) "NoCollision")
  (`PrimitiveComponent.SetSimulatePhysics` _hosetip false)
  (`PrimitiveComponent.SetCollisionEnabled` _hosetip "NoCollision")
  (bind _asmain_character (cast `MainCharacter` Instigator))
  (bind _output_get (set `self.Character` _asmain_character))
  (`InventoryComponent.AddItem` (`MainCharacter.GetInventory` _output_get) self))

(event `DropHose`
  (bind _hosetip (`self.HoseTip`))
  (`Interactable.StopInteract` null)
  (`PrimitiveComponent.SetSimulatePhysics` _hosetip true)
  (`PrimitiveComponent.SetCollisionEnabled` _hosetip "QueryAndPhysics")
  (`InventoryComponent.RemoveItem` (`MainCharacter.GetInventory` (`self.Character`)) self)
  (set `self.Character` null)
  (`KismetSystemLibrary.Delay` 0.2)
  (`PrimitiveComponent.SetCollisionEnabled` (`self.HermesInteractable`) "QueryOnly"))

(event `self.OnHolstered`
  (params (InInstigator :type "Controller Object Reference"))
  (`self.DropHose`))

(event `self.StopInteract`
  (params (InInstigator :type "Controller Object Reference"))
  (set `self.Interacting` false)
  (`ActorComponent.Deactivate` (`self.Niagara`)))

(event `self.ReceiveParticleData`
  (params (Data :type "Array of BasicParticleData Structure (by ref)") (NiagaraSystem :type "NiagaraSystem Object Reference") (SimulationPositionOffset :type "Vector Structure (by ref)"))
  (bind _pondref (`self.PondRef`))
  (bind (_origin _boxextent) (`KismetSystemLibrary.GetComponentBounds` (`/Game/Actors/Hose/BP_Pond.Box` _pondref)))
  (for _array_element Data
    (`|ExecutionSequence`
      (:`then_0`
        (if (not (`self.SkipParticle`))
          (`/Engine/EditorBlueprintResources/StandardMacros.IsValid` _pondref
            (:`Is Valid`
              (if (`FrogwaterStatics.IsPointInBox` (`.Position` (break `BasicParticleData` _array_element)) (`KismetMathLibrary.MakeBox` (- _origin _boxextent) (+ _origin _boxextent)))
                (`/Game/Actors/Hose/BP_Pond.Fill` (`self.PondRef`)))))))
      (:`then_1`
        (set `self.SkipParticle` (not (`self.SkipParticle`)))))))

(fn `Interact`
  (params (InInstigator :type "Controller Object Reference"))
  (returns (ReturnValue :type Boolean))
  (`/Engine/EditorBlueprintResources/StandardMacros.IsValid` (`self.Character`) ; We can assume that if we have a character reference, then the hose is picked up.
    (:`Is Valid`
      (set `self.Interacting` true)
      (`ActorComponent.Activate` (`self.Niagara`) true)
      (return true))))

(fn `InteractRequiresAiming`
  (returns (ReturnValue :type Boolean))
  (return false))

(fn `UserConstructionScript`
  (bind _cable (`self.Cable`))
  (set `CableComponent.CableLength` (- (`self.Length`) 100.0) _cable)
  (set `CableComponent.CableWidth` (`self.Width`) _cable)
  (bind _output_get (set `CableComponent.bEnableStiffness` (> (`self.Stiffness`) 0) _cable))
  (if _output_get
    (set `CableComponent.SolverIterations` (`self.Stiffness`) _cable))
  (`NiagaraComponent.SetNiagaraVariableObject` (`self.Niagara`) "User.BPCallback" self))
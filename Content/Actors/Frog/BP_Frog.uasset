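; Physics-driven frog actor that hops and turns at random intervals and can be picked up into the main character's inventory.
; Self-restarting timers trigger velocity-change impulses for jumps, while Tick interpolates yaw toward random targets between jumps, toggling angular damping.
; Moving to the offhand pauses this behavior; holstering resumes it and removes the frog from inventory.
; Meeting quest requirements destroys its Scannable component.
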(event `self.ReceiveBeginPlay`
  (`self.StartJumpTimer`))

(event `CancelJumpTimer`
  (`KismetSystemLibrary.K2_ClearAndInvalidateTimerHandle` (`self.JumpTimer`)))

(event `StartJumpTimer`
  (bind (_x _y) (`KismetMathLibrary.BreakVector2D` (`self.JumpTimeRange`)))
  (bind _returnvalue (`KismetSystemLibrary.K2_SetTimerDelegate` (delegate `Jump`) (`KismetMathLibrary.RandomFloatInRange` _x _y)))
  (set `self.JumpTimer` _returnvalue))

(event `Jump`
  (bind (_x _y) (`KismetMathLibrary.BreakVector2D` (`self.UpVelocityRange`)))
  (bind (_x_2 _y_2) (`KismetMathLibrary.BreakVector2D` (`self.ForwardVelocityRange`)))
  (set `self.bJumping` true)
  (`self.CancelRotation`)
  (`PrimitiveComponent.AddImpulse` (`self.StaticMesh`) (+ (* (* (`self.GetActorRightVector`) -1.0) (`KismetMathLibrary.RandomFloatInRange` _x_2 _y_2)) (* (`self.GetActorUpVector`) (`KismetMathLibrary.RandomFloatInRange` _x _y))) "None" true)
  (`KismetSystemLibrary.Delay` 1.0)
  (set `self.bJumping` false)
  (`self.StartJumpTimer`))

(event `self.ReceiveTick`
  (params (DeltaSeconds :type "Float (single-precision)"))
  (bind _returnvalue (`self.K2_GetActorRotation`))
  (bind _rotationtarget (`self.RotationTarget`))
  (if (not (`self.bHeld`))
    (if (not (`self.bJumping`))
      (if (`self.bRotating`)
        (`self.K2_SetActorRotation` (`KismetMathLibrary.RInterpTo` _returnvalue (`KismetMathLibrary.MakeRotator` (.roll _returnvalue) (.pitch _returnvalue) _rotationtarget) DeltaSeconds (`self.RotationSpeed`)) true)
        (if (`KismetMathLibrary.NearlyEqual_FloatFloat` (.yaw _returnvalue) _rotationtarget 1.0)
          (`self.CancelRotation`))
        (elif (not (`KismetSystemLibrary.K2_IsTimerActiveHandle` (`self.RotateTimer`)))
          (`self.SetNextRotationTimer`))))))

(event `CancelRotation`
  (set `self.bRotating` false)
  (`KismetSystemLibrary.K2_ClearAndInvalidateTimerHandle` (`self.RotateTimer`))
  (`PrimitiveComponent.SetAngularDamping` (`self.StaticMesh`) 40.0))

(event `SetNextRotationTimer`
  (bind (_x _y) (`KismetMathLibrary.BreakVector2D` (`self.RotateTimeRange`)))
  (bind _returnvalue (`KismetSystemLibrary.K2_SetTimerDelegate` (delegate `StartRotation`) (`KismetMathLibrary.RandomFloatInRange` _x _y)))
  (set `self.RotateTimer` _returnvalue))

(event `StartRotation`
  (bind _returnvalue (`KismetMathLibrary.RandomFloatInRange` 40.0 180.0))
  (bind (_returnvalue_roll _returnvalue_pitch _returnvalue_yaw) (`KismetMathLibrary.BreakRotator` (`self.K2_GetActorRotation`)))
  (set `self.bRotating` true)
  (set `self.RotationTarget` (+ _returnvalue_yaw (select `bool` (`KismetMathLibrary.RandomBool`) :`false` _returnvalue :`true` (* _returnvalue -1.0))))
  (`PrimitiveComponent.SetAngularDamping` (`self.StaticMesh`) 0.0))

(event `self.HermesInteractable.OnInteractionComplete`
  (params (Sender :type "HermesInteractableComponent Object Reference") (Instigator :type "Actor Object Reference"))
  (`PrimitiveComponent.SetCollisionEnabled` (`self.HermesInteractable`) "NoCollision")
  (bind _asmain_character (cast `MainCharacter` Instigator))
  (`InventoryComponent.AddItem` (`MainCharacter.GetInventory` _asmain_character) self))

(event `self.OnOffhand`
  (params (InInstigator :type "Controller Object Reference"))
  (set `self.bHeld` true)
  (`self.CancelJumpTimer`)
  (`PrimitiveComponent.SetAngularDamping` (`self.StaticMesh`) 5.0))

(event `self.OnHolstered`
  (params (InInstigator :type "Controller Object Reference"))
  (set `self.bHeld` false)
  (`self.StartJumpTimer`)
  (`PrimitiveComponent.SetCollisionEnabled` (`self.HermesInteractable`) "QueryOnly")
  (`PrimitiveComponent.SetAngularDamping` (`self.StaticMesh`) 0.0)
  (bind _asmain_character (cast `MainCharacter` (`Controller.K2_GetPawn` InInstigator)))
  (`InventoryComponent.RemoveItem` (`MainCharacter.GetInventory` _asmain_character) self))

(event `self.QuestReaction.OnRequirementsMet`
  (params (Sender :type "QuestReactionComponent Object Reference"))
  (`ActorComponent.K2_DestroyComponent` (`self.Scannable`)))

(fn `Interact`
  (params (InInstigator :type "Controller Object Reference"))
  (returns (ReturnValue :type Boolean))
  (return false))

(fn `InteractRequiresAiming`
  (returns (ReturnValue :type Boolean))
  (return false))

(fn `UserConstructionScript`)
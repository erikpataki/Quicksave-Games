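; BP_TestCamera is a test camera item that the player picks up into the inventory and holds to take pictures.
; Completing the interaction disables pickup collision, adds it to the MainCharacter's inventory and sets the owning pawn.
; Parent-class aim and offhand events are extended to attach it to the hand root with a distinct pose and material each, while holstering detaches it.
; Taking a picture only adds a debug print to the parent behavior.
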(event `self.InteractableComponent.OnInteractionComplete`
  (params (Sender :type "HermesInteractableComponent Object Reference") (Instigator :type "Actor Object Reference"))
  (`PrimitiveComponent.SetCollisionEnabled` (`self.InteractableComponent`) "NoCollision")
  (bind _asmain_character (cast `MainCharacter` Instigator))
  (`InventoryComponent.AddItem` (`MainCharacter.GetInventory` _asmain_character) self)
  (`PrimitiveComponent.SetCollisionEnabled` (`self.GetPickupCollisionComponent`) "NoCollision")
  (`self.SetOwningPawn` _asmain_character))

(event `self.OnPictureTaken`
  (params (bSuccess :type Boolean) (ScannableComponent :type "ScannableComponent Object Reference"))
  (`parent.OnPictureTaken` bSuccess ScannableComponent)
  (`KismetSystemLibrary.PrintString` "Cap"))

(event `self.OnAim`
  (params (InInstigator :type "Controller Object Reference"))
  (`parent.OnAim` InInstigator)
  (`self.K2_SetActorRelativeTransform` (`KismetMathLibrary.MakeTransform` (40.0 0.0 -15.0) (struct) (0.25 0.25 0.25)))
  (bind _asmain_character (cast `MainCharacter` (`Controller.K2_GetPawn` InInstigator)))
  (`self.K2_AttachToComponent` (`MainCharacter.GetHandRoot` _asmain_character) "None" "KeepRelative" "KeepRelative" "KeepRelative")
  (`PrimitiveComponent.SetMaterial` (`self.GetStaticMeshComponent`) 0 "/Game/FPWeapon/Materials/FirstPersonProjectileMaterial.FirstPersonProjectileMaterial"))

(event `self.OnOffhand`
  (params (InInstigator :type "Controller Object Reference"))
  (`parent.OnOffhand` InInstigator)
  (`self.K2_SetActorRelativeTransform` (`KismetMathLibrary.MakeTransform` (60.0 0.0 -30.0) (struct :`Pitch` -30.0) (0.25 0.25 0.25)))
  (bind _asmain_character (cast `MainCharacter` (`Controller.K2_GetPawn` InInstigator)))
  (`self.K2_AttachToComponent` (`MainCharacter.GetHandRoot` _asmain_character) "None" "KeepRelative" "KeepRelative" "KeepRelative")
  (`PrimitiveComponent.SetMaterial` (`self.GetStaticMeshComponent`) 0 "/Game/FPWeapon/Materials/BaseMaterial.BaseMaterial"))

(event `self.OnHolstered`
  (params (InInstigator :type "Controller Object Reference"))
  (`parent.OnHolstered` InInstigator)
  (`self.K2_DetachFromActor` "KeepRelative"))

(fn `UserConstructionScript`)
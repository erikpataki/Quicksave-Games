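; BP_MainCharacter_Test is a test player character that exercises interaction, quest, footstep and UI systems.
; The E key starts interaction through InteractorComponent, whose focus, start and completion events print debug text.
; It also prints quest IDs from QuestSubsystem add and complete events, and shows a WB_LoadPictureTest widget while 6 is held.
; The construction script registers left and right foot audio components and a test particle with FootstepsComponent.
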(event `Key|Six`
  (params (Key :type "Key Structure"))
  (:`Pressed`
    (bind _asplayer_controller (cast `PlayerController` (`self.GetController`)))
    (bind _returnvalue (`|CreateWidget` "/Game/CharacterTest/WB_LoadPictureTest.WB_LoadPictureTest_C" _asplayer_controller))
    (bind _output_get (set `self.Widget` _returnvalue))
    (`UserWidget.AddToPlayerScreen` _output_get 0))
  (:`Released`
    (`Widget.RemoveFromParent` (`self.Widget`))))

(event `self.ReceiveBeginPlay`
  (bind _returnvalue (subsystem `QuestSubsystem`))
  (add `QuestSubsystem.OnQuestAdded` _returnvalue (delegate `OnQuestAdded_Event_0`))
  (add `QuestSubsystem.OnQuestComplete` _returnvalue (delegate `OnQuestComplete_Event_0`)))

(event `OnQuestAdded_Event_0`
  (params (Quest :type "Quest Structure (by ref)"))
  (`KismetSystemLibrary.PrintString` (`KismetStringLibrary.Conv_NameToString` (`.QuestId` (break `Quest` Quest)))))

(event `OnQuestComplete_Event_0`
  (params (Quest :type "Quest Structure (by ref)"))
  (`KismetSystemLibrary.PrintString` (`KismetStringLibrary.Conv_NameToString` (`.QuestId` (break `Quest` Quest)))))

(event `Key|E`
  (params (Key :type "Key Structure"))
  (:`Pressed`
    (`HermesInteractorComponent.StartInteraction` (`self.InteractorComponent`))))

(event `self.InteractorComponent.OnFocus`
  (params (Sender :type "HermesInteractorComponent Object Reference") (InteractableComponent :type "HermesInteractableComponent Object Reference"))
  (`KismetSystemLibrary.PrintString` (`KismetTextLibrary.Conv_TextToString` (`HermesInteractableComponent.GetFocusText` InteractableComponent))))

(event `self.InteractorComponent.OnInteractionStarted`
  (params (Sender :type "HermesInteractorComponent Object Reference") (InteractableComponent :type "HermesInteractableComponent Object Reference"))
  (`KismetSystemLibrary.PrintString` (`KismetTextLibrary.Conv_TextToString` (`HermesInteractableComponent.GetInteractingText` InteractableComponent))))

(event `self.InteractorComponent.OnInteractionComplete`
  (params (Sender :type "HermesInteractorComponent Object Reference") (InteractableComponent :type "HermesInteractableComponent Object Reference"))
  (`KismetSystemLibrary.PrintString` "Picked up"))

(fn `UserConstructionScript`
  (bind _footstepscomponent (`self.FootstepsComponent`))
  (bind _test_footsteps (`self.Test_Footsteps`))
  (`BFFootstepsComponent.AddFootUsingComponents` _footstepscomponent (`self.RightFoot`) _test_footsteps)
  (`BFFootstepsComponent.AddFootUsingComponents` _footstepscomponent (`self.LeftFoot`) _test_footsteps))